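; Test Blueprint that exercises the advanced control flow nodes MultiBranch, ConditionalSequence and MultiConditionalSelect by printing their results.
; Each Tick, a ConditionalSequence gated by three output toggles calls a separate test function per node.
; The tests share the same Bool conditions and print with keys, the select test covering two sets of variables, one apparently vectors.
; Unconnected copies of the nodes remain in the EventGraph and never run.
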(event EventTick
  (params (DeltaSeconds :type Float%20%28single-precision%29))
  (|ConditionalSequence (Variables|Default|GetOutputBranch) (Variables|Default|GetOutputSequence) (Variables|Default|GetOutputSelect)
    (:CaseExec_0
      (CallFunction|TestMultiBranch))
    (:CaseExec_1
      (CallFunction|TestConditionalSequencce))
    (:CaseExec_2
      (CallFunction|TestMultiSelect))))

(fn ConstructionScript)

(fn TestMultiBranch
  (Development|PrintString "[Multi Branch]" true true "(R=0.000000,G=0.660000,B=1.000000,A=1.000000)" 0.1 "Branch")
  (|MultiBranch (Variables|Default|GetBool0) (Variables|Default|GetBool1) (Variables|Default|GetBool2) (Variables|Default|GetBool3)
    (:DefaultExec
      (Development|PrintString "Default" true true "(R=0.000000,G=0.660000,B=1.000000,A=1.000000)" 0.1 "BranchDefault"))
    (:CaseExec_0
      (Development|PrintString "0" true true "(R=0.000000,G=0.660000,B=1.000000,A=1.000000)" 0.1 "Branch0"))
    (:CaseExec_1
      (Development|PrintString "1" true true "(R=0.000000,G=0.660000,B=1.000000,A=1.000000)" 0.1 "Branch1"))
    (:CaseExec_2
      (Development|PrintString "2" true true "(R=0.000000,G=0.660000,B=1.000000,A=1.000000)" 0.1 "Branch2"))
    (:CaseExec_3
      (Development|PrintString "3" true true "(R=0.000000,G=0.660000,B=1.000000,A=1.000000)" 0.1 "Branch3"))))

(fn TestConditionalSequencce
  (Development|PrintString "[Conditional Sequencce]" true true "(R=0.000000,G=0.660000,B=1.000000,A=1.000000)" 0.1 "Sequence")
  (|ConditionalSequence (Variables|Default|GetBool0) (Variables|Default|GetBool1) (Variables|Default|GetBool2) (Variables|Default|GetBool3)
    (:DefaultExec
      (Development|PrintString "Default" true true "(R=0.000000,G=0.660000,B=1.000000,A=1.000000)" 0.1 "SequenceDefault"))
    (:CaseExec_0
      (Development|PrintString "0" true true "(R=0.000000,G=0.660000,B=1.000000,A=1.000000)" 0.1 "Sequence0"))
    (:CaseExec_1
      (Development|PrintString "1" true true "(R=0.000000,G=0.660000,B=1.000000,A=1.000000)" 0.1 "Sequence1"))
    (:CaseExec_2
      (Development|PrintString "2" true true "(R=0.000000,G=0.660000,B=1.000000,A=1.000000)" 0.1 "Sequence2"))
    (:CaseExec_3
      (Development|PrintString "3" true true "(R=0.000000,G=0.660000,B=1.000000,A=1.000000)" 0.1 "Sequence3"))))

(fn TestMultiSelect
  (Development|PrintString "[Multi Select]" true true "(R=0.000000,G=0.660000,B=1.000000,A=1.000000)" 0.1 "Select")
  (Development|PrintString (Utilities|String|ToString(Float) (|MultiConditionalSelect (Variables|Default|GetDefault) (Variables|Default|GetVar0) (Variables|Default|GetVar1) (Variables|Default|GetVar2) (Variables|Default|GetVar3) (Variables|Default|GetBool0) (Variables|Default|GetBool1) (Variables|Default|GetBool2) (Variables|Default|GetBool3))) true true "(R=0.000000,G=0.660000,B=1.000000,A=1.000000)" 2.0 "SelectOut")
  (Development|PrintString (Utilities|String|ToString(Vector) (|MultiConditionalSelect (Variables|Default|GetDefaultVec) (Variables|Default|GetVec0) (Variables|Default|GetVec1) (Variables|Default|GetVec2) (Variables|Default|GetVec3) (Variables|Default|GetBool0) (Variables|Default|GetBool1) (Variables|Default|GetBool2) (Variables|Default|GetBool3))) true true "(R=0.000000,G=0.660000,B=1.000000,A=1.000000)" 2.0 "SelectOut2"))